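; BP_BasicStaticEnemy is an enemy Blueprint that fires projectiles.
; It extends the inherited Shoot event, calling the parent and then spawning a BP_Projectile at its Scene component's world transform, with itself as owner and its Target passed in.
; A leftover debug "Hello" prints after each shot, while BeginPlay is disabled and the construction script only calls the parent.
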(event EventBeginPlay
  (|CallParentFunction) ; This node is disabled and will not be called.\nDrag off pins to build functionality.
)

(event EventShoot
  (|CallParentFunction)
  (Game|SpawnActorfromClass "/Game/Blueprint/BP_Projectile.BP_Projectile_C" (Transformation|GetWorldTransform (Variables|Default|GetScene)) "AlwaysSpawn" "MultiplyWithRoot" self (Variables|Default|GetTarget) 0)
  (Development|PrintString "Hello"))

(fn ConstructionScript
  (|CallParentFunction))