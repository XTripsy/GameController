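; BP_Player is a player Blueprint that moves steadily along +X with layered sprite parallax.
; On BeginPlay, each Paper sprite under the Parallax component gets a dynamic material instance, with its ParallaxMultiplier parameter set from an array by layer index.
; A very short looping timer, rather than Tick, nudges the capsule forward by a fixed step without sweeping for collision.
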(event Custom|Set
  (bind _self self)
  (bind _playercapsulecomponent (Variables|Default|GetPlayerCapsuleComponent _self))
  (bind _output_get (Variables|Default|SetLoc (+ (Transformation|GetWorldLocation _playercapsulecomponent) "0.200000,0.000000,0.000000")))
  (Transformation|SetWorldLocation _playercapsulecomponent _output_get false false))

(event Custom|Set%20Parallax
  (for (_array_element _array_index) (Components|GetChildrenComponents (Variables|Default|GetParallax) false)
    (bind _aspaper_sprite_component (Utilities|Casting|CastToPaperSpriteComponent _array_element))
    (bind _returnvalue (Rendering|Material|CreateDynamicMaterialInstance _aspaper_sprite_component 0 0 "None" :!class /Script/Engine.PrimitiveComponent))
    (Utilities|Array|Add (Variables|Default|GetMaterialInstance) _returnvalue)
    (Rendering|Material|SetScalarParameterValue _returnvalue "ParallaxMultiplier" (Utilities|Array|Get(acopy) (Variables|Default|GetParallaxMultiplier) _array_index) :!class /Script/Engine.MaterialInstanceDynamic)))

(event EventBeginPlay
  (CallFunction|SetParallax)
  (Variables|Default|SetLoc (Transformation|GetWorldLocation (Variables|Default|GetPlayerCapsuleComponent self)))
  (Utilities|Time|SetTimerbyEvent (delegate Custom|Set) 0.001 true))

(fn ConstructionScript)