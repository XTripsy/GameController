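; Gameplay game mode that keeps flying enemies spawning around the player.
; A looping timer started on BeginPlay spawns a BP_FlyEnemyBase, while the live count is below MaxEnemy, at a random X offset on either side of the player pawn and slightly above it.
; Each enemy's Health OnDeath event is bound to decrement the count, freeing a slot for a later spawn.
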(event Custom|Spawn
  (bind _returnvalue (Game|Player|GetPlayerPawn 0))
  (bind _returnvalue_2 (Transformation|GetActorTransform _returnvalue))
  (Development|PrintString "Spawn")
  (if (< (Variables|Default|GetEnemyCount) (Variables|Default|GetMaxEnemy))
    (bind _returnvalue_3 (Game|SpawnActorfromClass "/Game/Blueprint/BP_FlyEnemyBase.BP_FlyEnemyBase_C" (Math|Transform|MakeTransform (+ (.location _returnvalue_2) (Math|Vector|MakeVector (CallFunction|RandomFloatwithNegate 4e+02 1e+03) 0.0 5e+01)) (.rotation _returnvalue_2) (.scale _returnvalue_2)) "AlwaysSpawn" "MultiplyWithRoot" 0 0))
    (bind _result (Math|Integer|IncrementInt (Variables|Default|GetEnemyCount))
      (:%20%20
        (Development|PrintString (Utilities|String|ToString(Integer) _result))
        (EventDispatchers|BindEventtoOnDeath (Variables|/Game/Blueprint/BP_BaseEnemy.BP_BaseEnemy_C|GetHealth _returnvalue_3) (delegate Custom|OnEnemyDeath))))))

(event Custom|OnEnemyDeath
  (Math|Integer|DecrementInt (Variables|Default|GetEnemyCount)))

(event EventBeginPlay
  (|CallParentFunction)
  (Utilities|Time|SetTimerbyEvent (delegate Custom|Spawn) 5.0 true))

(fn ConstructionScript)

(fn RandomFloatwithNegate
  (params (Min :type Float%20%28double-precision%29) (Max :type Float%20%28double-precision%29))
  (bind _returnvalue (Math|Random|RandomFloatinRange Min Max))
  (if (Math|Random|RandomBool)
    (return _returnvalue)
    (else
      (return (* _returnvalue -1.0)))))