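; Base enemy Blueprint for a launcher that aims and fires at the player while they are inside its detection box.
; Box overlaps set the target and pause or resume two looping timers, one for rotation and one at the fire rate.
; Aiming is pitch-only, computed from the X/Z offset to the target; Shoot is an empty event, apparently left for children.
; Any damage from a Projectile-tagged causer destroys the enemy.
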(event OnComponentBeginOverlap(Box)
  (params (OverlappedComponent :type Primitive%20Component%20Object%20Reference) (OtherActor :type Actor%20Object%20Reference) (OtherComp :type Primitive%20Component%20Object%20Reference) (OtherBodyIndex :type Integer) (bFromSweep :type Boolean) (SweepResult :type Hit%20Result%20Structure%20%28by%20ref%29))
  ;[1 1 1] Overlap
  (if (Actor|ActorHasTag OtherActor "Player")
    (Variables|Default|SetTarget OtherActor)
    (Utilities|Time|UnpauseTimerbyHandle (Variables|Default|GetShootTimer))
    (Utilities|Time|UnpauseTimerbyHandle (Variables|Default|GetRotationTImer))))

(event OnComponentEndOverlap(Box)
  (params (OverlappedComponent :type Primitive%20Component%20Object%20Reference) (OtherActor :type Actor%20Object%20Reference) (OtherComp :type Primitive%20Component%20Object%20Reference) (OtherBodyIndex :type Integer))
  (if (Actor|ActorHasTag OtherActor "Player")
    (Utilities|Time|PauseTimerbyHandle (Variables|Default|GetShootTimer))
    (Utilities|Time|PauseTimerbyHandle (Variables|Default|GetRotationTImer))))

(event Custom|Rotate
  (Transformation|SetWorldRotation (Variables|Default|GetLouncher) (Math|Rotator|MakeRotator 0.0 (CallFunction|GetPitchRotation) 0.0) false false))

(event Custom|Shoot)

(event Game|Damage|EventAnyDamage
  (params (Damage :type Float%20%28single-precision%29) (DamageType :type Damage%20Type%20Object%20Reference) (InstigatedBy :type Controller%20Object%20Reference) (DamageCauser :type Actor%20Object%20Reference))
  (if (Actor|ActorHasTag DamageCauser "Projectile")
    (Actor|DestroyActor)
    (Development|PrintString "Hello")))

(event EventBeginPlay
  (bind _returnvalue (Utilities|Time|SetTimerbyEvent (delegate Custom|Rotate) 0.05 true))
  (Utilities|Time|PauseTimerbyHandle _returnvalue)
  (Variables|Default|SetRotationTImer _returnvalue)
  (bind _returnvalue_2 (Utilities|Time|SetTimerbyEvent (EventDispatchers|CreateEvent :!event Custom|Shoot) (Variables|Default|GetFireRate) true))
  (Utilities|Time|PauseTimerbyHandle _returnvalue_2)
  (Variables|Default|SetShootTimer _returnvalue_2))

(fn ConstructionScript)

(fn GetPitchRotation
  (bind _target (Variables|Default|GetTarget))
  (bind _louncher (Variables|Default|GetLouncher))
  (bind _returnvalue (Transformation|GetActorLocation _target))
  (bind _returnvalue_2 (Transformation|GetWorldLocation _louncher))
  (bind _returnvalue_3 (- _returnvalue _returnvalue_2))
  (return (+ (* (Class|KismetMathLibrary|DegAtan2 (.x _returnvalue_3) (.z _returnvalue_3)) -1.0) 1e+01)))