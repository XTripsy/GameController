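; BP_FlyEnemyBase is a base Blueprint for a flying enemy that chases the player.
; On BeginPlay it sets the GCPlayer pawn's capsule as the homing target of its ProjectileMovement component, so projectile homing drives the pursuit.
; Hit events only produce debug output: a box drawn at the impact point and a "BUMP" print when the other actor has the Player tag.
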(event Collision|EventHit
  (params (MyComp :type Primitive%20Component%20Object%20Reference) (Other :type Actor%20Object%20Reference) (OtherComp :type Primitive%20Component%20Object%20Reference) (bSelfMoved :type Boolean) (HitLocation :type Vector :default "0, 0, 0") (HitNormal :type Vector :default "0, 0, 0") (NormalImpulse :type Vector :default "0, 0, 0") (Hit :type Hit%20Result%20Structure%20%28by%20ref%29))
  (Rendering|Debug|DrawDebugBox HitLocation "50.000000,50.000000,50.000000" "(R=1.000000,G=0.000000,B=0.002570,A=1.000000)" "0, 0, 0" 1.0 0.0)
  (if (Actor|ActorHasTag Other "Player")
    (Development|PrintString "BUMP")))

(event EventBeginPlay
  (|CallParentFunction)
  (bind _asgcplayer (Utilities|Casting|CastToGCPlayer (Game|Player|GetPlayerPawn 0)))
  (Variables|/Script/Engine.ProjectileMovementComponent|SetHomingTargetComponent (Variables|Default|GetProjectileMovement) (Variables|/Script/GameController.GCPlayer|GetPlayerCapsuleComponent _asgcplayer)))

(fn ConstructionScript)