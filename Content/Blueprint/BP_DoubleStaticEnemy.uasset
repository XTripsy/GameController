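; BP_DoubleStaticEnemy is an enemy Blueprint that fires two projectiles per shot.
; Its Shoot event loops over two spawn point components and spawns a BP_Projectile at each one's world transform, owned by the enemy and ignoring collisions.
; Nothing in this graph triggers Shoot, and the construction script only calls the parent's.
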(event EventBeginPlay
  (|CallParentFunction) ; This node is disabled and will not be called.\nDrag off pins to build functionality.
)

(event EventShoot
  (for _array_element (Utilities|Array|MakeArray (Variables|Default|GetProjectileSpawnPoint1) (Variables|Default|GetProjectileSpawnPoint))
    (Game|SpawnActorfromClass "/Game/Blueprint/BP_Projectile.BP_Projectile_C" (Transformation|GetWorldTransform _array_element) "AlwaysSpawn" "MultiplyWithRoot" self 0 0)))

(fn ConstructionScript
  (|CallParentFunction))