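; BP_StaticEnemy is an enemy Blueprint that fires projectiles at a target.
; Its Shoot event calls the parent implementation, then spawns a BP_Projectile at the ProjectileSpawnPoint transform with itself as owner, passing Target through.
; The spawn ignores collisions, and each shot prints the enemy's display name to the screen.
; The construction script only calls the parent.
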(event EventShoot
  (|CallParentFunction)
  (Game|SpawnActorfromClass "/Game/Blueprint/BP_Projectile.BP_Projectile_C" (Transformation|GetWorldTransform (Variables|Default|GetProjectileSpawnPoint)) "AlwaysSpawn" "MultiplyWithRoot" self (Variables|Default|GetTarget) 0)
  (Development|PrintString (Utilities|GetDisplayName self)))

(fn ConstructionScript
  (|CallParentFunction))