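; BP_Projectile is a projectile Blueprint with a Paper2D flipbook that damages actors tagged Player on hit.
; On BeginPlay it starts a self-destruct timer that destroys it after LifeDuration.
; Flipbook hits apply fixed damage, credited to the projectile's owner, without destroying the projectile.
; A separate misspelled DestoryActor event, not called within this Blueprint, only hides the actor after a short delay.
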(event OnComponentHit(PaperFlipbook)
  (params (HitComponent :type Primitive%20Component%20Object%20Reference) (OtherActor :type Actor%20Object%20Reference) (OtherComp :type Primitive%20Component%20Object%20Reference) (NormalImpulse :type Vector :default "0, 0, 0") (Hit :type Hit%20Result%20Structure%20%28by%20ref%29))
  (if (Actor|ActorHasTag OtherActor "Player")
    (Game|Damage|ApplyDamage 0 1e+01 0 (Components|GetOwner) "/Script/Engine.DamageType")))

(event Custom|AutoDestroyActor
  (Utilities|FlowControl|Delay (Variables|Default|GetLifeDuration))
  (Actor|DestroyActor))

(event Custom|DestoryActor
  (Utilities|FlowControl|Delay 0.2)
  (Rendering|SetActorHiddenInGame true))

(event EventBeginPlay
  (CallFunction|AutoDestroyActor))

(fn ConstructionScript)